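; AC_Shooter is a basic hitscan shooting Blueprint that fires on a left mouse click.
; Shoot runs a complex line trace on the Visibility channel from the player camera along its forward vector.
; It then draws a temporary debug box at the impact point without checking for a hit, and applies no damage or other effect.
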(event Custom|Shoot
  (bind _returnvalue (Game|GetPlayerCameraManager 0))
  (bind _returnvalue_2 (Camera|GetCameraLocation _returnvalue))
  (bind _outhit (Collision|LineTraceByChannel _returnvalue_2 (+ _returnvalue_2 (* (Transformation|GetActorForwardVector _returnvalue) 1e+04)) "TraceTypeQuery1" true 0 "None"))
  (Rendering|Debug|DrawDebugBox (.ImpactPoint (Collision|BreakHitResult _outhit)) "1.000000,1.000000,1.000000" "(R=0.094480,G=1.000000,B=0.000000,A=1.000000)" "0, 0, 0" 1e+01 1e+01))

(event EventBeginPlay
  (bind _returnvalue (Game|GetPlayerController 0))
  (Input|EnableInput _returnvalue _returnvalue))

(event Input|MouseEvents|LeftMouseButton
  (params (Key :type Key%20Structure :default "None"))
  (:Pressed
    (CallFunction|Shoot)))